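; BP_Enemy is a melee enemy that chases the first player character and punches it when in range.
; An AI MoveTo call restarts itself on success or failure for continuous pursuit.
; Overlapping the AttackRadius component starts a delayed recursive loop that plays a punch, applies damage and spawns Niagara effects while the player remains valid.
; Incoming damage reduces Health and enables mesh physics at zero, without stopping the chase or attack logic.
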(event OnComponentBeginOverlap(AttackRadius)
  (params (OverlappedComponent :type Primitive%20Component%20Object%20Reference) (OtherActor :type Actor%20Object%20Reference) (OtherComp :type Primitive%20Component%20Object%20Reference) (OtherBodyIndex :type Integer) (bFromSweep :type Boolean) (SweepResult :type Hit%20Result%20Structure%20%28by%20ref%29))
  ;[1 1 1] Attack Player
  (Utilities|Casting|CastToBP_ThirdPersonCharacter OtherActor)
  (Variables|Default|SetInAttackRadius true)
  (CallFunction|AttackPlayer))

(event OnComponentEndOverlap(AttackRadius)
  (params (OverlappedComponent :type Primitive%20Component%20Object%20Reference) (OtherActor :type Actor%20Object%20Reference) (OtherComp :type Primitive%20Component%20Object%20Reference) (OtherBodyIndex :type Integer))
  ;[1 1 1] Attack Player
  (Utilities|Casting|CastToBP_ThirdPersonCharacter OtherActor)
  (Variables|Default|SetInAttackRadius false))

(event Custom|Chase%20Player
  (AI|AIMoveTo self "0, 0, 0" (Game|GetPlayerCharacter 0) 3.0 false
    (:OnSuccess
      _)
    (:OnFail
      _))
  (CallFunction|ChasePlayer))

(event Custom|Attack%20Player
  (bind _returnvalue (Game|GetPlayerCharacter 0))
  ;[1 1 1] Attack Player
  (bind _asbp_third_person_character (Utilities|Casting|CastToBP_ThirdPersonCharacter _returnvalue))
  (if (and (Variables|Default|GetInAttackRadius) (>= (Variables|/Game/ThirdPerson/Blueprints/BP_ThirdPersonCharacter.BP_ThirdPersonCharacter_C|GetHealth _asbp_third_person_character) 0.0))
    (Components|Animation|PlayAnimation (Variables|Character|GetMesh) "/Game/AS_Punch.AS_Punch" false)
    (Game|Damage|ApplyDamage _returnvalue 1e+01 0 0)
    (Niagara|SpawnSystematLocation "/Game/NiagaraSystems/NS_DoDamage.NS_DoDamage" (.location (Transformation|GetActorTransform)))
    (Utilities|FlowControl|Delay 0.5)
    (CallFunction|AttackPlayer)))

(event EventBeginPlay
  (CallFunction|ChasePlayer))

(event Collision|EventActorBeginOverlap
  (params (OtherActor :type Actor%20Object%20Reference)))

(event EventTick
  (params (DeltaSeconds :type Float%20%28single-precision%29)))

(event Game|Damage|EventAnyDamage
  (params (Damage :type Float%20%28single-precision%29) (DamageType :type Damage%20Type%20Object%20Reference) (InstigatedBy :type Controller%20Object%20Reference) (DamageCauser :type Actor%20Object%20Reference))
  (bind _output_get (Variables|Default|SetHealth (- (Variables|Default|GetHealth) Damage)))
  (Niagara|SpawnSystematLocation "/Game/NiagaraSystems/NS_Damage.NS_Damage" (Transformation|GetActorLocation))
  (if (<= _output_get 0.0)
    (Physics|SetSimulatePhysics (Variables|Character|GetMesh) true)))

(fn ConstructionScript)